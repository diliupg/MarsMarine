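; Player-controlled marine pawn with world-axis movement and twin-stick style aiming.
; Each tick it aims by thumbstick or mouse, depending on whether the last key pressed was a gamepad key.
; Past a deadzone, stick angle sets control yaw directly, while mouse movement direction, rather than cursor position, steers it with smoothed interpolation.
; Fire input only activates and deactivates the assault rifle muzzle flash component.
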(event `InputAxis|Move_Forward_Backward`
  (params (AxisValue :type "Float (single-precision)"))
  (`self.AddMovementInput` (1.0 0.0 0.0) AxisValue))

(event `InputAxis|Move_Right_Left`
  (params (AxisValue :type "Float (single-precision)"))
  (`self.AddMovementInput` (0.0 1.0 0.0) AxisValue))

(event `self.ReceiveTick`
  (params (DeltaSeconds :type "Float (single-precision)"))
  (`self.UpdatePlayerAim`))

(event `Key|AnyKey`
  (params (Key :type "Key Structure"))
  (:`Pressed`
    (set `self.GamepadActive` (`KismetInputLibrary.Key_IsGamepadKey` Key))))

(event `InputAction|Fire`
  (params (Key :type "Key Structure"))
  (:`Pressed`
    (`self.StartFireWeapon`))
  (:`Released`
    (`self.EndFireWeapon`)))

(fn `EndFireWeapon`
  (`ActorComponent.Deactivate` (`self.P_AssaultRifle_MF`)))

(fn `Get Thumbstick Aim Direction`
  (returns (ReturnValue :type "Rotator Structure"))
  (return (`KismetMathLibrary.MakeRotator` 0.0 0.0 (`KismetMathLibrary.DegAtan2` (`self.GetInputAxisValue`) (`self.GetInputAxisValue`)))))

(fn `GetMouseAimDirection`
  (returns (ReturnValue :type "Rotator Structure"))
  (bind (_returnvalue_x _returnvalue_y) (`KismetMathLibrary.BreakVector2D` (`self.GetMouseVelocity`)))
  (return (`KismetMathLibrary.RInterpTo` (`Controller.GetControlRotation` (`GameplayStatics.GetPlayerController` 0)) (`KismetMathLibrary.MakeRotator` 0.0 0.0 (`KismetMathLibrary.DegAtan2` _returnvalue_y _returnvalue_x)) (`GameplayStatics.GetWorldDeltaSeconds`) (`self.Mouse Smoothing Strength`))))

(fn `GetMouseVelocity`
  (returns (ReturnValue :type "Vector2D Structure"))
  (bind (_deltax _deltay) (`PlayerController.GetInputMouseDelta` (`GameplayStatics.GetPlayerController` 0)))
  (return (/ (`KismetMathLibrary.MakeVector2D` _deltax _deltay) (`GameplayStatics.GetWorldDeltaSeconds`))))

(fn `IsMouseAboveDeadzone`
  (returns (ReturnValue :type Boolean))
  (return (> (`KismetMathLibrary.VSize2D` (`self.GetMouseVelocity`)) (`self.MouseDeadzone`))))

(fn `IsThumbstickAboveDeadzone`
  (returns (ReturnValue :type Boolean))
  (return (> (`KismetMathLibrary.VSize2D` (`KismetMathLibrary.MakeVector2D` (`self.GetInputAxisValue`) (`self.GetInputAxisValue`))) (`self.ThumbstickDeadzone`))))

(fn `StartFireWeapon`
  (`ActorComponent.Activate` (`self.P_AssaultRifle_MF`) false))

(fn `Update Thumbstick Aim`
  (if (`self.IsThumbstickAboveDeadzone`)
    (`Controller.SetControlRotation` (`GameplayStatics.GetPlayerController` 0) (`self.Get Thumbstick Aim Direction`))))

(fn `UpdateMouseAim`
  (if (`self.IsMouseAboveDeadzone`)
    (`Controller.SetControlRotation` (`GameplayStatics.GetPlayerController` 0) (`self.GetMouseAimDirection`))))

(fn `UpdatePlayerAim`
  (locals (MouseSmoothingStrength :type "Float (double-precision)" :default 10.0))
  (if (`self.GamepadActive`)
    (`self.Update Thumbstick Aim`)
    (else
      (`self.UpdateMouseAim`))))

(fn `UserConstructionScript`)