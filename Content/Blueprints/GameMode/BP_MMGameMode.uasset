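; Game mode that runs wave-based alien spawning for a marine player.
; A looping timer started after BeginPlay spawns BP_Alien actors at random TargetPoints until the current wave's quota from AliensInEachWave is reached.
; BP_Alien calls AreAllAliensDead after a death, which compares the marine's PlayerKills with the spawned count.
; On a match, StartNewWave waits, advances the wave, zeroes the spawn count and restarts the timer.
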(event `self.ReceiveBeginPlay`
  (`KismetSystemLibrary.Delay` 2.0)
  (`self.SetupNewWave`))

(event `SpawnWave`
  (`self.SpawnAlien`)
  (`self.Stop SpawningAliensIfLimitReached`))

(event `EndWave`
  (`KismetSystemLibrary.Delay` 2.0)
  (`self.SetupNewWave`))

(event `StartNewWave`
  (`KismetSystemLibrary.Delay` 5.0)
  (`/Engine/EditorBlueprintResources/StandardMacros.IncrementInt` (`self.CurrentWave`)
    (:`  `
      ;[1 1 1] At start of each wave we Zero this
      (set `self.AliensAddedToLevel` 0)
      (`self.SetupNewWave`))))

(fn `AreAllAliensDead`
  ;[1 1 1] This function is called from the BP_Alien soon after an Alien death to check is all Aliens are dead
  (bind _asbp_marine (cast `/Game/Blueprints/Pawns/BP_Marine` (`GameplayStatics.GetPlayerCharacter` 0)))
  (if (== (`/Game/Blueprints/Pawns/BP_Marine.PlayerKills` _asbp_marine) (`self.AliensAddedToLevel`))
    (`self.StartNewWave`)))

(fn `GetRandomSpawnPoints`
  (returns (SpawnPoint :type "TargetPoint Object Reference"))
  (bind _outactors (`GameplayStatics.GetAllActorsOfClass` "/Script/Engine.TargetPoint"))
  (return (`|GetArrayItem` _outactors (`KismetMathLibrary.RandomIntegerInRange` 0 (`KismetArrayLibrary.Array_LastIndex` _outactors)))))

(fn `SetupNewWave`
  (`KismetSystemLibrary.K2_SetTimer` null "SpawnWave" (`self.SpawnFrequency`) true))

(fn `SpawnAlien`
  (bind _spawnpoint (`self.GetRandomSpawnPoints`))
  (`/Engine/EditorBlueprintResources/StandardMacros.IsValid` _spawnpoint
    (:`Is Valid`
      (`|SpawnActorFromClass` "/Game/Blueprints/AI/BP_Alien.BP_Alien_C" (`self.GetTransform` _spawnpoint) "Undefined" "OverrideRootScale" null null)
      (`/Engine/EditorBlueprintResources/StandardMacros.IncrementInt` (`self.AliensAddedToLevel`)))))

(fn `Stop SpawningAliensIfLimitReached`
  (if (== (`self.AliensAddedToLevel`) (`|GetArrayItem` (`self.AliensInEachWave`) (`self.CurrentWave`)))
    (`KismetSystemLibrary.K2_ClearTimer` null "SpawnWave")))

(fn `UserConstructionScript`)