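; BP_Alien is an enemy AI character that chases the player, attacks in melee range and takes damage.
; While alive, it repeats AIMoveTo on the player, four seconds after each success or failure.
; Tick checks range, then pauses movement for a random attack montage; DamagePlayer applies the hit but is not called here.
; At zero health it stops, disables collision, credits a BP_Marine kill and is destroyed after a delay.
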(event `self.ReceiveBeginPlay`
  ;[1 1 1] AI Movement
  (if (`self.IsAlive`) :!label _label
    (`|AIMoveTo` self (0.0 0.0 0.0) (`GameplayStatics.GetPlayerCharacter` 0)
      (:`OnSuccess`
        _)
      (:`OnFail`
        _))
    (`KismetSystemLibrary.Delay` 4.0)
    (goto _label)))

(event `self.ReceiveTick`
  (params (DeltaSeconds :type "Float (single-precision)"))
  (bind _animmontages (`self.AnimMontages`))
  ;[1 1 1] AI Attack Code
  (if (`self.CanAttack`)
    (set `self.AnimIsPlaying` true)
    (`self.DeactivateAIMovement`)
    (`|PlayMontage` (`self.Mesh`) (`|GetArrayItem` _animmontages (`KismetMathLibrary.RandomInteger` (`KismetArrayLibrary.Array_Length` _animmontages)))
      (:`OnCompleted`
        (`self.ActivateAIMovement`)
        (set `self.AnimIsPlaying` false)))))

(event `self.ReceiveAnyDamage`
  (params (Damage :type "Float (single-precision)") (DamageType :type "DamageType Object Reference") (InstigatedBy :type "Controller Object Reference") (DamageCauser :type "Actor Object Reference"))
  ;[1 1 1] Damage and Destroy AI
  (if (`self.IsAlive`)
    (bind _health (`self.DecreaseHealth` Damage))
    (if (== _health 0.0)
      (`self.KillAI`)
      (`KismetSystemLibrary.Delay` 3.0)
      (`self.K2_DestroyActor`))))

(fn `ActivateAIMovement`
  (`ActorComponent.Activate` (`self.CharacterMovement`) false))

(fn `CanAttack`
  (returns (ReturnValue :type Boolean))
  (return (and (not (`self.AnimIsPlaying`)) (`self.IsWithinAttackRange`) (`self.IsAlive`))))

(fn `DamagePlayer`
  (if (`self.IsAlive`)
    (`GameplayStatics.ApplyDamage` (`GameplayStatics.GetPlayerCharacter` 0) (`self.DamagePerHit`))))

(fn `DeactivateAIMovement`
  (bind _charactermovement (`self.CharacterMovement`))
  (`MovementComponent.StopMovementImmediately` _charactermovement)
  (`ActorComponent.Deactivate` _charactermovement))

(fn `DecreaseHealth`
  (params (DecreaseAmount :type "Float (double-precision)"))
  (returns (Health :type "Float (double-precision)"))
  (bind _output_get (set `self.EnemyHealth` (`KismetMathLibrary.FClamp` (- (`self.EnemyHealth`) DecreaseAmount) 0.0 100.0)))
  (return _output_get))

(fn `IsAlive`
  (returns (ReturnValue :type Boolean))
  (return (not (`self.Dead`))))

(fn `IsAttacking`
  (returns (`return Value` :type Boolean))
  (return (`AnimInstance.Montage_IsPlaying` (`SkeletalMeshComponent.GetAnimInstance` (`self.Mesh`)) "/Game/Characters/Enemy_Great_Spider/Animations/AM_AlienAttack1.AM_AlienAttack1")))

(fn `IsWithinAttackRange`
  (returns (`return Value` :type Boolean))
  (return (< (`self.GetDistanceTo` (`GameplayStatics.GetPlayerCharacter` 0)) (`self.AttackRange`))))

(fn `KillAI`
  (set `self.Dead` true)
  (`self.DeactivateAIMovement`)
  (`self.SetActorEnableCollision` false)
  (bind _asbp_marine (cast `/Game/Blueprints/Pawns/BP_Marine` (`GameplayStatics.GetPlayerPawn` 0)))
  (`/Game/Blueprints/Pawns/BP_Marine.IncreaseKills` _asbp_marine))

(fn `UserConstructionScript`)